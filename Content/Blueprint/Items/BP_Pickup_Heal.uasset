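; Health pickup that heals BP_MainCharacter and can optionally grant a max health bonus.
; Actor overlap heals the character by HealAmount and destroys the pickup.
; OnPicked separately heals by HealAmount0 and, if ApplyMaxHealthIncrease is set, adds MaxHealthIncrease through TopDownPlayerState.
; The OnPicked path does not destroy the actor itself, and the overlap path never applies the bonus.
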(event `self.ReceiveActorBeginOverlap`
  (params (OtherActor :type "Actor Object Reference"))
  (bind _asbp_main_character (cast `/Game/Characters/BP_MainCharacter` OtherActor))
  (`MainCharacter.Heal` _asbp_main_character (`self.HealAmount`))
  (`self.K2_DestroyActor`))

(fn `OnPicked`
  (params (InstigatorPawn :type "Pawn Object Reference"))
  (returns (ReturnValue :type Boolean))
  (bind _asbp_main_character (cast `/Game/Characters/BP_MainCharacter` InstigatorPawn))
  (`MainCharacter.Heal` _asbp_main_character (`self.HealAmount_0`))
  (if (`self.bApplyMaxHealthIncrease`)
    (bind _astop_down_player_state (cast `TopDownPlayerState` (`Controller.PlayerState` (`Pawn.GetController` _asbp_main_character))))
    (`TopDownPlayerState.AddMaxHealthBonus` _astop_down_player_state (`self.MaxHealthIncrease`))
    (return false)))

(fn `UserConstructionScript`)