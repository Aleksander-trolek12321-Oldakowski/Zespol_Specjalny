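; BP_BaseWeapon is a base weapon Blueprint with empty Shoot and EndShoot events and shared hitscan logic.
; CreateShotTrace runs a multi line trace for Pawns from ShotArrow along its forward vector over a given Range.
; Each hit Enemy_MeleeGreatSword takes Damage through its Attributes and refreshes its HP widget.
; The GunShots sound plays in 2D only when the trace hits nothing.
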(event `Shoot`)

(event `EndShoot`)

(event `CreateShotTrace`
  (params (Range :type "Float (double-precision)"))
  (bind _shotarrow (`self.ShotArrow`))
  (bind _returnvalue (`SceneComponent.K2_GetComponentLocation` _shotarrow))
  (bind (_outhits _returnvalue_2) (`KismetSystemLibrary.LineTraceMultiForObjects` _returnvalue (+ _returnvalue (* (`KismetMathLibrary.GetForwardVector` (`SceneComponent.K2_GetComponentRotation` _shotarrow)) Range)) (`|MakeArray` "ObjectTypeQuery3" :!type "EObjectTypeQuery Enum")))
  (if _returnvalue_2
    (for _array_element _outhits
      (bind (_bblockinghit _binitialoverlap _time _distance _location _impactpoint _normal _impactnormal _physmat _hitactor) (`GameplayStatics.BreakHitResult` _array_element))
      (bind _asenemy_melee_great_sword (cast `Enemy_MeleeGreatSword` _hitactor))
      (`AttributesComponent.ApplyDamage` (`EnemyBase.Attributes` _asenemy_melee_great_sword) (`self.Damage`))
      (bind _asenemy_melee_great_sword_2 (cast `Enemy_MeleeGreatSword` _hitactor))
      (`EnemyBase.UpdateHPWidget` _asenemy_melee_great_sword_2))
    (else
      (`GameplayStatics.PlaySound2D` (`self.GunShots`) 1.0 1.0 0.0 null null))))

(fn `UserConstructionScript`)